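; BP_WallBuilder is an actor that builds a modular wall from a row of static mesh pieces.
; The construction script adds WallPieces components at fixed intervals along local X, then assigns each a mesh from the Meshes array.
; Mesh picks use a random stream from Seed, so layouts are repeatable.
; RandomizeWall rerolls the seed, then randomizes existing meshes before calling GenerateWall, which adds another set of pieces.
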(event `RandomizeWall`
  (set `self.Seed` (`KismetMathLibrary.RandomIntegerInRange` 0 64000))
  (`self.RandomizeMeshes`)
  (`self.GenerateWall`))

(event `GenerateWall`
  (for _index (range (`self.WallPieces`))
    (`AddComponent|NODE_AddStaticMeshComponent-1` :`RelativeTransform` (`KismetMathLibrary.MakeTransform` (`KismetMathLibrary.MakeVector` (`KismetMathLibrary.Conv_IntToDouble` (* _index 400)))))))

(event `RandomizeMeshes`
  (set `self.Stream` (`KismetMathLibrary.MakeRandomStream` (`self.Seed`)))
  (for _array_element (`self.K2_GetComponentsByClass` "/Script/Engine.StaticMeshComponent")
    (`StaticMeshComponent.SetStaticMesh` _array_element (`KismetArrayLibrary.Array_RandomFromStream` (`self.Meshes`) (`self.Stream`)))))

(fn `UserConstructionScript`
  (locals (NewLocalVar :type "StaticMesh Object Reference"))
  (`self.GenerateWall`)
  (`self.RandomizeMeshes`))