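; BP_ProceduralWall is an actor that builds a straight wall from a configurable number of randomly chosen mesh pieces.
; Its construction script adds static mesh components at fixed spacing along X, then assigns each a mesh from the Meshes array.
; Picks come from a random stream seeded by InitialSeed, so layouts stay repeatable.
; RandomizeWall rolls a new seed and reassigns the meshes.
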(event `GenerateWall`
  (for _index (range (`self.WallPieceCount`))
    (`AddComponent|NODE_AddStaticMeshComponent-1` :`RelativeTransform` (`KismetMathLibrary.MakeTransform` (`KismetMathLibrary.MakeVector` (`KismetMathLibrary.Conv_IntToDouble` (* _index 400)))))))

(event `RandomizeMeshes`
  (set `self.RandomStream` (`KismetMathLibrary.MakeRandomStream` (`self.Initial Seed`)))
  (for _array_element (`self.K2_GetComponentsByClass` "/Script/Engine.StaticMeshComponent")
    (`StaticMeshComponent.SetStaticMesh` _array_element (`KismetArrayLibrary.Array_RandomFromStream` (`self.Meshes`) (`self.RandomStream`)))))

(event `RandomizeWall`
  (set `self.Initial Seed` (`KismetMathLibrary.RandomIntegerInRange` 0 64000))
  (`self.RandomizeMeshes`))

(fn `UserConstructionScript`
  (`self.GenerateWall`)
  (`self.RandomizeMeshes`))